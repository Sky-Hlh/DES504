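; BP_starParticleRlease is a star particle effect actor that feeds the player's position into its particle system.
; On BeginPlay it sets two vector parameters on the ParticleSystem component: pointlocation from the player character mesh's world location and pointlocation1 from the character's actor location.
; Both values are sampled only once, since Tick is empty and the construction script does nothing.
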(event `self.ReceiveBeginPlay`
  (bind _returnvalue (`GameplayStatics.GetPlayerCharacter` 0))
  (`ParticleSystemComponent.SetVectorParameter` (`self.ParticleSystem`) "pointlocation" (`SceneComponent.K2_GetComponentLocation` (`Character.Mesh` _returnvalue)))
  (`ParticleSystemComponent.SetVectorParameter` (`self.ParticleSystem`) "pointlocation1" (`self.K2_GetActorLocation` _returnvalue)))

(event `self.ReceiveTick`
  (params (DeltaSeconds :type "Float (single-precision)")))

(fn `UserConstructionScript`)